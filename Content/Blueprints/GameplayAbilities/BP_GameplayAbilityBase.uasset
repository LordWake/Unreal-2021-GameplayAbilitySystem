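; Base gameplay ability Blueprint providing shared helpers for cost checks and UI cooldown feedback.
; GetPlayerInfo resolves the owning BP_CharacterBase and, when it has one, its player controller.
; DoUICoolDown starts the cooldown on primary UI slots whose ability class matches this ability's info.
; IsCostStillAvailable negates the configured cost and checks that the character's matching Health, Mana or Strength attribute exceeds it.
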(fn GetPlayerInfo
  ;[0 1 0.954] Returns the PlayerCharacter and the PlayerController
  (bind _asbp_character_base (Utilities|Casting|CastToBP_CharacterBase (Ability|GetOwningActorfromActorInfo)))
  (bind _asbp_player_controller_base (Utilities|Casting|CastToBP_PlayerControllerBase (Pawn|GetController _asbp_character_base))
    (:then
      _)
    (:CastFailed
      _))
  (return _asbp_character_base _asbp_player_controller_base))

(fn DoUICoolDown
  ;[0 1 0.8074] Updates Abilities UI Cooldown
  (bind _playercontrollerbase (CallFunction|GetPlayerInfo))
  (Utilities|IsValid _playercontrollerbase
    (:Is%20Valid
      (bind _aswbp_primary_ui (Utilities|Casting|CastToWBP_PrimaryUI (Variables|/Script/AbilitySystem.PlayerControllerBase|GetUIReference _playercontrollerbase)))
      (for _array_element (Variables|/Game/UI/Blueprints/WBP_PrimaryUI.WBP_PrimaryUI_C|GetSlots _aswbp_primary_ui)
        (bind _returnvalue (Class|GameplayAbilityBase|GetAbilityInfo))
        (if (== (.abilityclass _returnvalue) (.abilityclass (Variables|/Game/UI/Blueprints/WBP_Ability_Slot.WBP_Ability_Slot_C|GetAbilityInfo _array_element)))
          (Default|StartCoolDown _array_element))))))

(fn IsCostStillAvailable
  (bind _returnvalue (Class|GameplayAbilityBase|GetAbilityInfo))
  (LocalVariables|SetValueCost (* (.cost _returnvalue) -1.0))
  (switch Utilities|FlowControl|Switch|SwitchonEAbilityCostType (.costtype _returnvalue)
    (:Health
      (bind _characterbase (CallFunction|GetPlayerInfo))
      (return (> (.currentvalue (Variables|/Script/AbilitySystem.AttributeSetBase|GetHealth (Variables|/Script/AbilitySystem.CharacterBase|GetBaseAttributeSetComponent _characterbase))) (LocalVariables|GetValueCost))))
    (:Mana
      (bind _characterbase_2 (CallFunction|GetPlayerInfo))
      (return (> (.currentvalue (Variables|/Script/AbilitySystem.AttributeSetBase|GetMana (Variables|/Script/AbilitySystem.CharacterBase|GetBaseAttributeSetComponent _characterbase_2))) (LocalVariables|GetValueCost))))
    (:Strength
      (bind _characterbase_3 (CallFunction|GetPlayerInfo))
      (return (> (.currentvalue (Variables|/Script/AbilitySystem.AttributeSetBase|GetStrength (Variables|/Script/AbilitySystem.CharacterBase|GetBaseAttributeSetComponent _characterbase_3))) (LocalVariables|GetValueCost))))))