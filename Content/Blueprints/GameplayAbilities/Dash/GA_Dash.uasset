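; GA_Dash is a Gameplay Ability that launches the character forward with a dash montage, damaging and knocking back targets.
; On activation it commits, starts the UI cooldown, pushes the character and switches its collision to overlap.
; Skill.Dash.DealDamage events apply GE_Dash_Damage and push the target away from the owner with a stun.
; Any montage exit restores ground friction and blocking collision, then ends the ability.
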(event Ability|EventActivateAbility
  (Ability|CommitAbility)
  ;[0.9368 1 0] Updates Cooldown on UI
  (CallFunction|DoUICoolDown)
  (bind _characterbase (CallFunction|GetPlayerInfo))
  (Variables|Default|SetOriginalGroundFriction (Variables|/Script/Engine.CharacterMovementComponent|GetGroundFriction (Variables|/Script/Engine.Character|GetCharacterMovement _characterbase)))
  ;[0.03139 1 0] Make the dash by pushing the character and playing an Animation Montage
  (Class|CharacterBase|PushCharacter _characterbase (Transformation|GetActorForwardVector _characterbase) 3e+03 0.0)
  (bind _characterbase_2 (CallFunction|GetPlayerInfo))
  (Class|CharacterBase|SetNewCollision _characterbase_2 "ECR_Overlap")
  (|PlayMontageandWaitProxy "None" "/Game/Blueprints/Characters/Animation/AM_ShinbiDash.AM_ShinbiDash" 1.0 "None" true 1.0
    (:then
      ;[0 1 0.4853] Aplplies GameplayEffect Damage to enemies
      (bind _payload (Ability|Tasks|WaitGameplayEvent "(TagName=\"Skill.Dash.DealDamage\")" 0)
        (:EventReceived
          (GameplayEffects|ApplyGameplayEffectToTarget (Ability|TargetData|AbilityTargetDatafromActor (.Target (Utilities|Struct|BreakGameplayEventData _payload))) "/Game/Blueprints/GameplayAbilities/Dash/GE_Dash_Damage.GE_Dash_Damage_C" 1 1)
          (bind _asbp_character_base (Utilities|Casting|CastToBP_CharacterBase (.Target (Utilities|Struct|BreakGameplayEventData _payload))))
          (Class|CharacterBase|PushCharacter _asbp_character_base (Math|Vector|Normalize (- (Transformation|GetActorLocation _asbp_character_base) (Transformation|GetActorLocation (Ability|GetOwningActorfromActorInfo)))) 3e+03 2.0))))
    (:OnCompleted
      ;[0 1 0.2453] Finish the Ability Execution and set everything to default values
      (Variables|/Script/Engine.CharacterMovementComponent|SetGroundFriction (Variables|/Script/Engine.Character|GetCharacterMovement _characterbase_2) (Variables|Default|GetOriginalGroundFriction) :!label _label)
      (bind _characterbase_3 (CallFunction|GetPlayerInfo))
      (Class|CharacterBase|SetNewCollision _characterbase_3 "ECR_Block")
      (Ability|EndAbility))
    (:OnBlendOut
      (goto _label))
    (:OnInterrupted
      (goto _label))
    (:OnCancelled
      (goto _label))))