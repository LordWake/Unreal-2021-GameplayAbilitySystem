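; Ground Blast gameplay ability: a player-aimed area attack that damages targets and launches characters into the air.
; After a cost check, it plays a targeting montage, enables camera-controlled rotation and awaits user confirmation through BP_GATargetActorGroundSelect.
; Confirmation commits the ability, starts UI cooldown and plays the cast montage, spawning particles, applying damage and pushing characters upward with a stun.
; Camera-controlled rotation is switched off after pushes and when the ability ends.
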(event Ability|EventActivateAbility
  ;[1 0.887 0] Checks if we have enought mana like to start casting this Ability
  (bind _bcan (CallFunction|IsCostStillAvailable))
  (if _bcan
    ;[0 1 0.9497] Cast the Ability and waits for PlayerInputs. Meanwhile, it'll keep repeating the Animation
    (|PlayMontageandWaitProxy "None" "/Game/Blueprints/Characters/Animation/AM_GroundBlast_Targeting.AM_GroundBlast_Targeting" 1.0 "None" true 1.0
      (:then
        (Utilities|FlowControl|Delay (Variables|/Script/Engine.AnimSequenceBase|GetSequenceLength (Animation|GetCurrentMontage :!class /Script/GameplayAbilities.GameplayAbility)))
        (bind _characterbase (CallFunction|GetPlayerInfo))
        (Class|CharacterBase|MakeCameraControlRotation _characterbase true)
        ;[1 0.4299 0.976] When we have the Target Confirmed, then it will Play the other Montage, Spawn Emitters, and Apply damage to all the enemies inside the Collision Sphere (Check C++ GATargetActorGroundSelect)
        (bind _data (|WaitTargetData :ConfirmationType "UserConfirmed" :Class "/Game/Blueprints/GameplayAbilities/GroundBlast/BP_GATargetActorGroundSelect.BP_GATargetActorGroundSelect_C" :ReticleClass 0)
          (:ValidData
            (bind _characterbase_2 (CallFunction|GetPlayerInfo))
            (Variables|/Script/AbilitySystem.CharacterBase|SetbIsTargeting _characterbase_2 false)
            (Ability|CommitAbility)
            (CallFunction|DoUICoolDown)
            (|PlayMontageandWaitProxy "None" "/Game/Blueprints/Characters/Animation/AM_GroundBlast_Cast.AM_GroundBlast_Cast" 1.0 "None" true 1.0
              (:then
                (Effects|SpawnEmitteratLocation "/Game/Blueprints/GameplayAbilities/GroundBlast/P_GroundBlast.P_GroundBlast" (Class|AbilitySystemBlueprintLibrary|GetTargetDataEndPoint _data (- (Ability|TargetData|GetDataCountfromTargetData _data) 1)))
                (GameplayEffects|ApplyGameplayEffectToTarget _data "/Game/Blueprints/GameplayAbilities/GroundBlast/GE_GroundBlast_Damage.GE_GroundBlast_Damage_C" 1 1)
                ;[0.1859 1 0] Push all the Characters to the air.
                (for _array_element (Ability|TargetData|GetActorsfromTargetData _data)
                  (bind _asbp_character_base (Utilities|Casting|CastToBP_CharacterBase _array_element))
                  (Class|CharacterBase|PushCharacter _asbp_character_base "0, 0,1.000000" 5e+02 2.0 "/Game/Blueprints/Characters/Animation/AM_GroundBlast_InAir.AM_GroundBlast_InAir")
                  (Utilities|FlowControl|Delay 0.2)
                  (bind _characterbase_3 (CallFunction|GetPlayerInfo))
                  (Class|CharacterBase|MakeCameraControlRotation _characterbase_3 false)))
              (:OnCompleted
                (Ability|EndAbility :!label _label))
              (:OnBlendOut
                (goto _label))
              (:OnInterrupted
                (goto _label))
              (:OnCancelled
                (goto _label))))
          (:Cancelled
            (Ability|EndAbility)))))
    (else
      (Ability|EndAbility))))

(event Ability|EventOnEndAbility
  (params (bWasCancelled :type Boolean))
  (bind _characterbase (CallFunction|GetPlayerInfo))
  (Class|CharacterBase|MakeCameraControlRotation _characterbase false))