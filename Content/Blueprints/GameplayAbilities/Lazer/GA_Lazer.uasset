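; GA_Lazer is a Gameplay Ability that casts a continuous, mana-draining laser from the character.
; After the casting montage starts, it attaches BP_Lazer to a mesh socket and switches the character to camera-driven rotation for aiming.
; BP_Lazer sends overlapped actors through gameplay events, which apply damage and stunning knockback while the cost remains affordable, otherwise ending the ability.
; Ending removes the draining cost, destroys the laser and restores rotation.
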(event Ability|EventActivateAbility
  (Ability|CommitAbility)
  (CallFunction|DoUICoolDown)
  (|PlayMontageandWaitProxy "None" "/Game/Blueprints/Characters/Animation/AM_LazerCasting.AM_LazerCasting" 1.0 "None" true 1.0
    (:then
      (Utilities|FlowControl|Delay 0.3)
      (bind _characterbase (CallFunction|GetPlayerInfo))
      ;[1 0.4018 0] Spawn Lazer and change the actors movement rotation so we can orient the laser to the Camera rotation
      (bind _spawnedactor (|SpawnActor :Class "/Game/Blueprints/GameplayAbilities/Lazer/BP_Lazer.BP_Lazer_C" :Instigator _characterbase)
        (:then
          (bind _output_get (Variables|Default|SetLazerActor _spawnedactor))
          (Transformation|AttachComponentToComponent _output_get (Variables|/Script/Engine.Character|GetMesh _characterbase) "Lazer" "SnapToTarget" "SnapToTarget" "KeepRelative" true)
          (Class|CharacterBase|MakeCameraControlRotation _characterbase true)
          ;[0.2503 1 0.9245] The BP_Lazer pass all the overlaped actor through this Gameplay Event Data, then, we apply damage to the enemies
          (bind _payload (Ability|Tasks|WaitGameplayEvent "(TagName=\"Skill.Lazer.DealDamage\")" 0)
            (:EventReceived
              (bind _bcan (CallFunction|IsCostStillAvailable))
              (if _bcan
                (GameplayEffects|ApplyGameplayEffectToTarget (.TargetData (Utilities|Struct|BreakGameplayEventData _payload)) "/Game/Blueprints/GameplayAbilities/Lazer/GE_LazerDamage.GE_LazerDamage_C" 1 1)
                (for _array_element (Ability|TargetData|GetActorsfromTargetData (.TargetData (Utilities|Struct|BreakGameplayEventData _payload)))
                  (bind _asbp_character_base (Utilities|Casting|CastToBP_CharacterBase _array_element))
                  (Class|CharacterBase|PushCharacter _asbp_character_base (Math|Vector|Normalize (- (Transformation|GetActorLocation _asbp_character_base) (Transformation|GetWorldLocation (Variables|/Game/Blueprints/GameplayAbilities/Lazer/BP_Lazer.BP_Lazer_C|GetLazerEndDetector (.AsBP%20Lazer (Utilities|Casting|CastToBP_Lazer (Variables|Default|GetLazerActor))))))) 5e+02 0.3 "/Game/Blueprints/Characters/Animation/AM_HitStun.AM_HitStun"))
                (else
                  (Ability|EndAbility))))))))))

(event Ability|EventOnEndAbility
  (params (bWasCancelled :type Boolean))
  ;[0 1 0] Remove the draining cost when finish this Ability. Otherwise, is gonna keep consuming Mana forever.
  (Ability|RemoveGameplayEffectFromOwnerWithAssetTags "(GameplayTags=((TagName=\"Skill.Lazer.DrainingCost\")))")
  (Actor|DestroyActor (Variables|Default|GetLazerActor))
  (bind _characterbase (CallFunction|GetPlayerInfo))
  (Class|CharacterBase|MakeCameraControlRotation _characterbase false))