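; BP_CharacterBase is the shared character Blueprint that turns collision overlaps into melee and dash attack damage events for its gameplay abilities.
; Sword collider overlaps send a Skill.Melee.DealDamage gameplay event to itself, with the overlapped character as target, when that character reports it as hostile.
; Capsule overlaps send Skill.Dash.DealDamage the same way, recording each enemy in an exclusion list so it is not signaled again.
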(event OnComponentBeginOverlap(SwordCollider)
  (params (OverlappedComponent :type Primitive%20Component%20Object%20Reference) (OtherActor :type Actor%20Object%20Reference) (OtherComp :type Primitive%20Component%20Object%20Reference) (OtherBodyIndex :type Integer) (bFromSweep :type Boolean) (SweepResult :type Hit%20Result%20Structure%20%28by%20ref%29))
  (bind _self self)
  ;[1 0 0] Sword Attack Ability
  (if (!= OtherActor self)
    (bind _asbp_character_base (Utilities|Casting|CastToBP_CharacterBase OtherActor))
    (bind _returnvalue (Class|CharacterBase|IsOtherHostile _asbp_character_base _self))
    (if _returnvalue
      (Ability|SendGameplayEventtoActor _self "(TagName=\"Skill.Melee.DealDamage\")" (Utilities|Struct|MakeGameplayEventData "" _self OtherActor)))))

(event OnComponentBeginOverlap(CapsuleComponent)
  (params (OverlappedComponent :type Primitive%20Component%20Object%20Reference) (OtherActor :type Actor%20Object%20Reference) (OtherComp :type Primitive%20Component%20Object%20Reference) (OtherBodyIndex :type Integer) (bFromSweep :type Boolean) (SweepResult :type Hit%20Result%20Structure%20%28by%20ref%29))
  (bind _self self)
  ;[0 1 0] Dash Attack Ability
  (bind _asbp_character_base (Utilities|Casting|CastToBP_CharacterBase OtherActor))
  (bind _returnvalue (Class|CharacterBase|IsOtherHostile _asbp_character_base _self))
  (if _returnvalue
    (bind _returnvalue_2 (Class|CharacterBase|EnemyIsAlreadyExcluded _asbp_character_base))
    (if (not _returnvalue_2)
      (Utilities|Array|AddUnique (Variables|Default|GetOverlapExclude) _asbp_character_base)
      (Ability|SendGameplayEventtoActor self "(TagName=\"Skill.Dash.DealDamage\")" (Utilities|Struct|MakeGameplayEventData "" _self OtherActor)))))

(fn ConstructionScript)