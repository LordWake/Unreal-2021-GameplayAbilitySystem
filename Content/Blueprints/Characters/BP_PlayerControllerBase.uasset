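; Base player controller Blueprint that links the primary UI's ability slots to the controlled character's Gameplay Ability System.
; It forwards granted ability info to the UI and maps five slot events to one shared activation function.
; That function reads the slot's class from the UI and tries to activate it on the pawn.
; It then flags targeting for BP_GameplayTarget classes, cancels targeting and clears the combo.
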(event EventAddAbilitytoUI
  (params (AbilityInfo :type Gameplay%20Ability%20Info%20Structure))
  ;[0 0 1] Add Abilities to the UI
  (bind _aswbp_primary_ui (Utilities|Casting|CastToWBP_PrimaryUI (Variables|Default|GetUIReference)))
  (Default|AddAbilitytoSlots _aswbp_primary_ui AbilityInfo))

(event EventSlotOneAbilityUI
  ;[1 0.06016 0.6167] Call Abilities from Slot UI class
  (CallFunction|TryActivateAbilityinUISlot))

(event EventSlotTwoAbilityUI
  ;[1 0.06016 0.6167] Call Abilities from Slot UI class
  (CallFunction|TryActivateAbilityinUISlot 1))

(event EventSlotThreeAbilityUI
  ;[1 0.06016 0.6167] Call Abilities from Slot UI class
  (CallFunction|TryActivateAbilityinUISlot 2))

(event EventSlotFourAbilityUI
  ;[1 0.06016 0.6167] Call Abilities from Slot UI class
  (CallFunction|TryActivateAbilityinUISlot 3))

(event EventSlotFiveAbilityUI
  ;[1 0.06016 0.6167] Call Abilities from Slot UI class
  (CallFunction|TryActivateAbilityinUISlot 4))

(fn ConstructionScript)

(fn TryActivateAbilityinUISlot
  (params (AbilitySlot :type Integer))
  ;[1 0 0.6888] Here we check for the Slot Ability we are calling, if it is valid. This function is called from the PlayerControllerInputs
  (bind _aswbp_primary_ui (Utilities|Casting|CastToWBP_PrimaryUI (Variables|Default|GetUIReference)))
  (bind (_ability_class _isvalid) (Default|GetSlotAbilityClass _aswbp_primary_ui AbilitySlot))
  (if _isvalid
    (bind _asbp_character_base (Utilities|Casting|CastToBP_CharacterBase (Pawn|GetControlledPawn)))
    ;[0 1 0] And if everything works fine, we activate that ability from our character AbilitySystem Component.
    (Abilities|TryActivateAbilitybyClass (Ability|GetAbilitySystemComponent _asbp_character_base) _ability_class true)
    ;[0 1 0.4223] Depends on our targeting, we can decide if make a melee attack or a Targeting class like GroundBlast.
    (Utilities|Casting|CastToBP_GameplayTargetClass _ability_class
      (:then
        (Variables|/Script/AbilitySystem.CharacterBase|SetbIsTargeting _asbp_character_base true))
      (:CastFailed
        (Variables|/Script/AbilitySystem.CharacterBase|SetbIsTargeting _asbp_character_base false)))
    ;[1 0 0] And cancel the target so if we change between abilities, there is no TargetData. Otherwise, you'll be able to still see GroundBlast Decal
    (Class|AbilitySystemComponent|TargetCancel (Ability|GetAbilitySystemComponent _asbp_character_base))
    (Class|CharacterBase|ClearCombo _asbp_character_base)))