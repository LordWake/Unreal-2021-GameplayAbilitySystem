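; Player character Blueprint that uses the Gameplay Ability System and feeds its attributes to the HUD.
; On BeginPlay it applies a basic regeneration gameplay effect to itself.
; Health, Mana and Strength change events reach WBP_PrimaryUI through the player controller's UI reference and set each matching glass ball to the current-to-max ratio.
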(event EventBeginPlay
  (GameplayEffects|ApplyGameplayEffectToSelf :self (Variables|Default|GetAbilitySystemComponent) :GameplayEffectClass "/Game/Blueprints/GameplayAbilities/GeneralGameplayEffects/GE_BasicRegen.GE_BasicRegen_C"))

(event EventOnHealthChanged
  (params (Health :type Float%20%28single-precision%29) (MaxHealth :type Float%20%28single-precision%29))
  ;[0 0.8079 1] Updates UI values for Health, Mana and Strength
  (bind _asbp_player_controller_base (Utilities|Casting|CastToBP_PlayerControllerBase (Pawn|GetController)))
  (bind _aswbp_primary_ui (Utilities|Casting|CastToWBP_PrimaryUI (Variables|/Script/AbilitySystem.PlayerControllerBase|GetUIReference _asbp_player_controller_base)))
  (Default|SetPercentage (Variables|/Game/UI/Blueprints/WBP_PrimaryUI.WBP_PrimaryUI_C|GetHealth_GlassBall _aswbp_primary_ui) (/ Health MaxHealth)))

(event EventOnManaChanged
  (params (Mana :type Float%20%28single-precision%29) (MaxMana :type Float%20%28single-precision%29))
  ;[0 0.8079 1] Updates UI values for Health, Mana and Strength
  (bind _asbp_player_controller_base (Utilities|Casting|CastToBP_PlayerControllerBase (Pawn|GetController)))
  (bind _aswbp_primary_ui (Utilities|Casting|CastToWBP_PrimaryUI (Variables|/Script/AbilitySystem.PlayerControllerBase|GetUIReference _asbp_player_controller_base)))
  (Default|SetPercentage (Variables|/Game/UI/Blueprints/WBP_PrimaryUI.WBP_PrimaryUI_C|GetMana_GlassBall _aswbp_primary_ui) (/ Mana MaxMana)))

(event EventOnStrengthChanged
  (params (Strength :type Float%20%28single-precision%29) (MaxStrength :type Float%20%28single-precision%29))
  ;[0 0.8079 1] Updates UI values for Health, Mana and Strength
  (bind _asbp_player_controller_base (Utilities|Casting|CastToBP_PlayerControllerBase (Pawn|GetController)))
  (bind _aswbp_primary_ui (Utilities|Casting|CastToWBP_PrimaryUI (Variables|/Script/AbilitySystem.PlayerControllerBase|GetUIReference _asbp_player_controller_base)))
  (Default|SetPercentage (Variables|/Game/UI/Blueprints/WBP_PrimaryUI.WBP_PrimaryUI_C|GetStrength_GlassBall _aswbp_primary_ui) (/ Strength MaxStrength)))

(fn ConstructionScript
  (|CallParentFunction))